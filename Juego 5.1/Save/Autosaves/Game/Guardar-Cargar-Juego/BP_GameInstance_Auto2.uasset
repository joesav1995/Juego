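; Game Instance that saves and loads the player's position through SaveGame slots.
; GuardarPartida writes the player pawn's transform to the "Partida 1" slot.
; CargarPartida teleports BP_FirstPersonCharacter to that transform, calls its CargarConfig and then MenuPrincipal, or creates the slot with an unset position if none exists.
; MenuPrincipal saves a false menu flag to its own "MenuPrincipal" slot.
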(event `GuardarPartida`
  (bind _returnvalue (`GameplayStatics.CreateSaveGameObject` "/Game/Guardar-Cargar-Juego/GuardarCargar.GuardarCargar_C"))
  (set `/Game/Guardar-Cargar-Juego/GuardarCargar.PosicionJugador` (`Actor.GetTransform` (`GameplayStatics.GetPlayerPawn` 0)) _returnvalue)
  (`GameplayStatics.SaveGameToSlot` _returnvalue "Partida 1")
  (`KismetSystemLibrary.PrintText` "Guardado"))

(event `CargarPartida`
  (bind _returnvalue (`GameplayStatics.DoesSaveGameExist` "Partida 1"))
  (if _returnvalue
    (bind _returnvalue_2 (`GameplayStatics.LoadGameFromSlot` "Partida 1"))
    (bind _asguardar_cargar (cast `/Game/Guardar-Cargar-Juego/GuardarCargar` _returnvalue_2))
    (bind _asbp_first_person_character (cast `/Game/FirstPerson/Blueprints/BP_FirstPersonCharacter` (`GameplayStatics.GetPlayerPawn` 0)))
    (`Actor.K2_SetActorTransform` _asbp_first_person_character (`/Game/Guardar-Cargar-Juego/GuardarCargar.PosicionJugador` _asguardar_cargar) false true)
    (`KismetSystemLibrary.PrintText` "Cargado")
    (`/Game/FirstPerson/Blueprints/BP_FirstPersonCharacter.CargarConfig` _asbp_first_person_character)
    (`self.MenuPrincipal`)
    (else
      (bind _returnvalue_3 (`GameplayStatics.CreateSaveGameObject` "/Game/Guardar-Cargar-Juego/GuardarCargar.GuardarCargar_C"))
      (set `/Game/Guardar-Cargar-Juego/GuardarCargar.PosicionJugador` (struct) _returnvalue_3)
      (`GameplayStatics.SaveGameToSlot` _returnvalue_3 "Partida 1"))))

(event `MenuPrincipal`
  (bind _returnvalue (`GameplayStatics.CreateSaveGameObject` "/Game/Guardar-Cargar-Juego/MenuPrincipal.MenuPrincipal_C"))
  (set `/Game/Guardar-Cargar-Juego/MenuPrincipal.MenuPrincipal` false _returnvalue)
  (`GameplayStatics.SaveGameToSlot` _returnvalue "MenuPrincipal")
  (`KismetSystemLibrary.PrintText` "Menu guardado"))